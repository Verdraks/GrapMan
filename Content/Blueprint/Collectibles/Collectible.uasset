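; Collectible pickup actor with a cube that spins around yaw each tick, scaled by Speed and frame time.
; When an actor of exactly the BP_Character class begins overlapping its Box, it sets IsPicked, fires OnCollect and disables itself.
; Enable and Disable events toggle visibility, component activation and Box collision, so the actor is hidden rather than destroyed; enabling leaves IsPicked unchanged.
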(event `EnableCollectible`
  (`self.SetActorHiddenInGame` false)
  (`ActorComponent.SetActive` (`self.Cube`) true false)
  (`ActorComponent.SetActive` (`self.Box`) true false)
  (`PrimitiveComponent.SetCollisionEnabled` (`self.Box`) "QueryOnly"))

(event `DisableCollectible`
  (`self.SetActorHiddenInGame` true)
  (`ActorComponent.SetActive` (`self.Box`) false false)
  (`ActorComponent.SetActive` (`self.Cube`) false false)
  (`PrimitiveComponent.SetCollisionEnabled` (`self.Box`) "NoCollision"))

(event `self.ReceiveTick`
  (params (DeltaSeconds :type "Float (single-precision)"))
  (`SceneComponent.K2_AddWorldRotation` (`self.Cube`) (`KismetMathLibrary.MakeRotator` 0.0 0.0 (* DeltaSeconds (`self.Speed`))) false false))

(event `self.Box.OnComponentBeginOverlap`
  (params (OverlappedComponent :type "PrimitiveComponent Object Reference") (OtherActor :type "Actor Object Reference") (OtherComp :type "PrimitiveComponent Object Reference") (OtherBodyIndex :type Integer) (bFromSweep :type Boolean) (SweepResult :type "HitResult Structure (by ref)"))
  (if (== (`GameplayStatics.GetObjectClass` OtherActor) "/Game/Blueprint/Character/BP_Character.BP_Character_C")
    (set `self.IsPicked` true)
    (`self.OnCollect`)
    (`self.DisableCollectible`)))

(fn `UserConstructionScript`)