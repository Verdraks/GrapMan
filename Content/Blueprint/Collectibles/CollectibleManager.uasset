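; Level manager that tracks picked collectibles, persists their state and opens the end menu once all are collected.
; On BeginPlay it restores picks from the game instance by collectible ID, disabling picked ones and binding to the rest.
; It broadcasts picked and total counts through a CollectiblesUpdate dispatcher.
; Completion also requires all collectibles from previous levels; EndPlay registers the ID-to-picked map back in the game instance.
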(event `self.ReceiveBeginPlay`
  (`self.LoadCollectibles`)
  (`KismetSystemLibrary.RetriggerableDelay` 0.05)
  (add `self.CollectiblesUpdate` (`|CreateDelegate` (`/Game/Blueprint/Character/BP_Controller.HUD` (cast `/Game/Blueprint/Character/BP_Controller` (`GameplayStatics.GetPlayerController` 0) :!pure true)) :!event `UpdateCollectiblesHUD`))
  (`self.CollectiblesUpdate` (`self.CollectiblesPicked`) (`KismetArrayLibrary.Array_Length` (`self.Collectibles`)))
  (set `self.GameInstance` (cast `/Game/Blueprint/BP_CustomGameInstance` (`GameplayStatics.GetGameInstance`) :!pure true)))

(event `self.ReceiveEndPlay`
  (params (EndPlayReason :type "EEndPlayReason Enum" :default "Destroyed"))
  (`self.SaveCollectibles`))

(event `OnCollectiblePickup`
  (bind _result (`/Engine/EditorBlueprintResources/StandardMacros.IncrementInt` (`self.CollectiblesPicked`))
    (:`  `
      (`self.CollectiblesUpdate` _result (`KismetArrayLibrary.Array_Length` (`self.Collectibles`)))
      (if (`self.CheckAllCollectiblesGetted`)
        (`GameplayStatics.OpenLevelBySoftObjectPtr` "/Game/Scene/EndMenu.EndMenu")))))

(fn `CheckAllCollectiblesGetted`
  (returns (AllAreCompleted :type Boolean))
  (locals (AllGetted :type Boolean))
  (if (`/Game/Blueprint/BP_CustomGameInstance.AllCollectibleCollectInPreviousLevel` (`self.GameInstance`))
    (set `local.AllGetted` true)
    (for _array_element (`self.Collectibles`)
      (if (not (`/Game/Blueprint/Collectibles/Collectible.IsPicked` _array_element))
        (set `local.AllGetted` false)
        (break)))
    (return (`local.AllGetted`))
    (else
      (return (`local.AllGetted`)))))

(fn `LoadCollectibles`
  (locals (Loaded :type Boolean))
  (bind _outactors (`GameplayStatics.GetAllActorsOfClass` "/Game/Blueprint/Collectibles/Collectible.Collectible_C"))
  (bind _output_get (set `self.Collectibles` _outactors))
  (bind (_datacollectibles _levelloaded) (`/Game/Blueprint/BP_CustomGameInstance.LoadDataLevel` (cast `/Game/Blueprint/BP_CustomGameInstance` (`GameplayStatics.GetGameInstance`) :!pure true)))
  (set `local.Loaded` _levelloaded)
  (for _array_element _output_get
    (if (`local.Loaded`)
      (bind (_value _returnvalue) (`BlueprintMapLibrary.Map_Find` (`.Collectibles_5_8965BF7D4F0BC67A2D93F6B4FBC2AC4F` (break `/Game/Blueprint/Collectibles/Struct_CollectibleData` _datacollectibles)) (`/Game/Blueprint/Collectibles/Collectible.ID` _array_element)))
      (if (and _value _returnvalue)
        (`/Game/Blueprint/Collectibles/Collectible.DisableCollectible` _array_element)
        (`/Engine/EditorBlueprintResources/StandardMacros.IncrementInt` (`self.CollectiblesPicked`))
        (else
          (add `/Game/Blueprint/Collectibles/Collectible.OnCollect` _array_element (`|CreateDelegate` :!event `OnCollectiblePickup`) :!label _label)))
      (else
        (goto _label)))))

(fn `SaveCollectibles`
  (locals (Data :type "Map of String to Boolean"))
  (for _array_element (`self.Collectibles`)
    (`BlueprintMapLibrary.Map_Add` (`local.Data`) (`/Game/Blueprint/Collectibles/Collectible.ID` _array_element) (`/Game/Blueprint/Collectibles/Collectible.IsPicked` _array_element)))
  (`/Game/Blueprint/BP_CustomGameInstance.RegisterDataLevel` (cast `/Game/Blueprint/BP_CustomGameInstance` (`GameplayStatics.GetGameInstance`) :!pure true) (make `/Game/Blueprint/Collectibles/Struct_CollectibleData` (`local.Data`))))

(fn `UserConstructionScript`)