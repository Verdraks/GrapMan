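; Custom Game Instance that keeps collectible data for each level across level changes during a play session.
; A map keyed by current level name holds the data: RegisterDataLevel writes the current level's entry, and LoadDataLevel returns it with a flag showing whether one was found.
; ClearGameInstance empties the map; nothing here saves it to disk.
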(fn `ClearGameInstance`
  (`BlueprintMapLibrary.Map_Clear` (`self.DataCollectibles`)))

(fn `LoadDataLevel`
  (returns (DataCollectibles :type "/Game/Blueprint/Collectibles/Struct_CollectibleData Structure") (LevelLoaded :type Boolean))
  (bind _returnvalue (`GameplayStatics.GetCurrentLevelName` true))
  (bind (_value _returnvalue_2) (`BlueprintMapLibrary.Map_Find` (`self.DataCollectibles`) _returnvalue))
  (return _value _returnvalue_2))

(fn `RegisterDataLevel`
  (params (DataCollectibles :type "/Game/Blueprint/Collectibles/Struct_CollectibleData Structure"))
  (bind _returnvalue (`GameplayStatics.GetCurrentLevelName` true))
  (`BlueprintMapLibrary.Map_Add` (`self.DataCollectibles`) _returnvalue DataCollectibles))