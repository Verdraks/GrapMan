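; Actor component that gives BP_ThirdPersonCharacter a grappling hook, pulling it toward a point hit by a camera-direction line trace.
; Launching switches movement to Flying, shows a cable component and starts a fast looping timer for the grapple update.
; The update pins the cable end to the hit point and applies an attraction force, skewed sideways by move input.
; Releasing restores Walking, hides the cable and clears the timer.
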(event `self.ReceiveBeginPlay`
  (bind _output_get (set `self.Owner` (cast `/Game/ThirdPerson/Blueprints/BP_ThirdPersonCharacter` (`self.GetOwner`) :!pure true)))
  (`/Engine/EditorBlueprintResources/StandardMacros.IsValid` (`self.GrappleHookMesh`)
    (:`Is Valid`
      _)
    (:`Is Not Valid`
      (bind _returnvalue (`|AddComponentByClass` :`self` _output_get :`Class` "/Script/CableComponent.CableComponent"))
      (bind _output_get_2 (set `self.GrappleHookMesh` _returnvalue))))
  (`self.SetVisibility` _output_get_2 false false))

(event `LaunchGrapplingHook`
  (bind _owner (`self.Owner`))
  (bind _returnvalue (`Actor.K2_GetActorLocation` _owner))
  (bind (_outhit _returnvalue_2) (`KismetSystemLibrary.LineTraceSingle` :`Start` _returnvalue :`End` (+ _returnvalue (* (`self.GetForwardVector` (`/Game/ThirdPerson/Blueprints/BP_ThirdPersonCharacter.FollowCamera` _owner)) (`self.RangeGrapple`))) :`TraceChannel` "TraceTypeQuery1" :`DrawDebugType` "ForDuration"))
  (if _returnvalue_2
    (set `self.IsGrappling` true)
    (set `self.GrapPoint` (`.ImpactPoint` (`GameplayStatics.BreakHitResult` _outhit)))
    (`CharacterMovementComponent.SetMovementMode` (`Character.CharacterMovement` (`self.Owner`)) "MOVE_Flying" 0)
    (`self.SetVisibility` (`self.GrappleHookMesh`) true false)
    (bind _returnvalue_3 (`KismetSystemLibrary.K2_SetTimerDelegate` (`|CreateDelegate` :!event `UpdateGrapplingHook`) 0.005 true true))
    (set `self.TimerEventUpdateGrappling` _returnvalue_3)))

(event `ReleaseGrapplingHook`
  (set `self.IsGrappling` false)
  (`CharacterMovementComponent.SetMovementMode` (`Character.CharacterMovement` (`self.Owner`)) "MOVE_Walking" 0)
  (`self.SetVisibility` (`self.GrappleHookMesh`) false false)
  (`KismetSystemLibrary.K2_ClearAndInvalidateTimerHandle` (`self.TimerEventUpdateGrappling`)))

(event `UpdateGrapplingHook`
  (bind _returnvalue_x (`KismetMathLibrary.BreakVector2D` (`|GetInputActionValue`)))
  (bind _owner (`self.Owner`))
  (set `CableComponent.EndLocation` (`KismetMathLibrary.InverseTransformLocation` (`Actor.GetTransform` (`self.Owner`)) (`self.GrapPoint`)) (`self.GrappleHookMesh`))
  (`CharacterMovementComponent.AddForce` (`Character.CharacterMovement` _owner) (* (`KismetMathLibrary.Normal` (+ (`KismetMathLibrary.GetDirectionUnitVector` (`Actor.K2_GetActorLocation` _owner) (`self.GrapPoint`)) (* (* (`Actor.GetActorRightVector` _owner) _returnvalue_x) (`self.ForceRotation`)))) (`self.AttractionForce`))))